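; BP_ObjectExportTool is a utility Blueprint that exports a static mesh or a camera to JSON files in the project Content directory.
; Two functions, ExportStaticMesh and ExportCamera, pass the StaticMesh variable or the Camera's CameraComponent to same-named export calls.
; Each output file takes the exported object's name plus a .json extension.
; The event graph and construction script are empty, so nothing runs automatically.
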(event EventBeginPlay)

(event Collision|EventActorBeginOverlap
  (params (OtherActor :type Actor%20Object%20Reference)))

(event EventTick
  (params (DeltaSeconds :type Float%20%28single-precision%29)))

(fn ConstructionScript)

(fn ExportStaticMesh
  (bind _staticmesh (Variables|Default|GetStaticMesh))
  (Class|ObjectExporterBPLibrary|ExportStaticMesh _staticmesh (Utilities|String|Append (Class|KismetSystemLibrary|GetProjectContentDirectory) (Utilities|GetObjectName _staticmesh) ".json")))

(fn ExportCamera
  (bind _camera (Variables|Default|GetCamera))
  (bind _cameracomponent (Variables|/Script/Engine.CameraActor|GetCameraComponent _camera))
  (Class|ObjectExporterBPLibrary|ExportCamera _cameracomponent (Utilities|String|Append (Class|KismetSystemLibrary|GetProjectContentDirectory) (Utilities|GetObjectName _cameracomponent) ".json")))